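; Dashing enemy character that hurts the player through its damage box overlap.
; Pawn sensing writes the seen player to the Blackboard, and a launchdash event launches it along its forward vector.
; Damage passes a DoOnce with no visible reset, so only the first hit lowers health.
; At zero health it enables mesh physics, clears CanSpawn and is destroyed after a short delay.
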(event OnSeePawn(PawnSensing)
  (params (Pawn :type Pawn%20Object%20Reference))
  (bind _self self)
  (bind _returnvalue (AI|GetAIController _self))
  (bind _returnvalue_2 (AI|GetBlackboard _returnvalue))
  (bind _asbp_third_person_character (Utilities|Casting|CastToBP_ThirdPersonCharacter Pawn))
  (AI|Components|Blackboard|SetValueasObject _returnvalue_2 (Utilities|Name|MakeLiteralName "Player") _asbp_third_person_character)
  (AI|Components|Blackboard|SetValueasBool _returnvalue_2 (Utilities|Name|MakeLiteralName "hasSeenPlayer") true))

(event OnComponentBeginOverlap(DamageBox)
  (params (OverlappedComponent :type Primitive%20Component%20Object%20Reference) (OtherActor :type Actor%20Object%20Reference) (OtherComp :type Primitive%20Component%20Object%20Reference) (OtherBodyIndex :type Integer) (bFromSweep :type Boolean) (SweepResult :type Hit%20Result%20Structure%20%28by%20ref%29))
  (bind _asbp_third_person_character (Utilities|Casting|CastToBP_ThirdPersonCharacter OtherActor))
  (if (== _asbp_third_person_character OtherActor)
    (CallFunction|AddHP -20 _asbp_third_person_character)))

(event Custom|launchdash
  (Character|LaunchCharacter (* (Transformation|GetActorForwardVector) (Variables|Default|GetDashdistance)) true true))

(event Game|Damage|EventAnyDamage
  (params (Damage :type Float%20%28single-precision%29) (DamageType :type Damage%20Type%20Object%20Reference) (InstigatedBy :type Controller%20Object%20Reference) (DamageCauser :type Actor%20Object%20Reference))
  (Utilities|FlowControl|DoOnce false
    (:Completed
      (bind _output_get (Variables|Default|Sethealth (- (Variables|Default|Gethealth) Damage)))
      (if (<= _output_get 0.0)
        (Physics|SetSimulatePhysics (Variables|Character|GetMesh) true)
        (Collision|SetCollisionEnabled (Variables|Character|GetMesh) "QueryAndPhysics")
        (Variables|Default|SetAIControllerClass "/Game/bluePrints/Actors/Enemigos/IADash/AI_Controller.AI_Controller_C")
        (Variables|Default|SetCanSpawn false)
        (Utilities|FlowControl|Delay 1.0)
        (Actor|DestroyActor)))))

(fn ConstructionScript)